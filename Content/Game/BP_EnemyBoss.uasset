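; Hippo boss enemy character that chases the player, leaps and stomps.
; Tick drives AIMoveTo plus a Delay-gated forward leap about every five seconds; landing shakes the camera and re-enables the Detection overlap.
; Detection plays the stomp and enables HitZone, but HitZone's overlap event is empty and its damage-and-knockback logic is disconnected.
; Damage reduces Health with a brief material flash, or at zero enables mesh physics and destroys the actor.
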(event `self.ReceiveBeginPlay`
  (`PrimitiveComponent.SetCollisionEnabled` (`self.HitZone`) "NoCollision"))

(event `self.ReceiveTick`
  (params (DeltaSeconds :type "Float (single-precision)"))
  (bind _returnvalue (`GameplayStatics.GetPlayerCharacter` 0))
  (bind (_returnvalue_x _returnvalue_y) (`KismetMathLibrary.BreakVector` (`self.K2_GetActorLocation` _returnvalue)))
  (bind (_returnvalue_x_2 _returnvalue_y_2) (`KismetMathLibrary.BreakVector` (* (`KismetMathLibrary.GetForwardVector` (`self.K2_GetActorRotation`)) 1000.0)))
  (`|ExecutionSequence`
    (:`then_0`
      (`|AIMoveTo` self (`KismetMathLibrary.MakeVector` _returnvalue_x _returnvalue_y) _returnvalue 100.0))
    (:`then_1`
      (`KismetSystemLibrary.Delay` 5.0)
      (`PrimitiveComponent.SetCollisionEnabled` (`self.Detection`) "NoCollision")
      (set `self.ShouldStomp` false)
      (`SkeletalMeshComponent.PlayAnimation` (`self.Mesh`) "/Game/Game/Meshes/TestHippo/HippoJump.HippoJump" false)
      (`KismetSystemLibrary.Delay` 0.5)
      (`self.LaunchCharacter` (`KismetMathLibrary.MakeVector` _returnvalue_x_2 _returnvalue_y_2 500.0))
      (`KismetSystemLibrary.Delay` 0.5)
      (set `self.ShouldStomp` true))))

(event `self.ReceiveAnyDamage`
  (params (Damage :type "Float (single-precision)") (DamageType :type "DamageType Object Reference") (InstigatedBy :type "Controller Object Reference") (DamageCauser :type "Actor Object Reference"))
  ;[1 1 1] Dégât reçu
  (`KismetSystemLibrary.Delay` 0.1)
  (set `self.Health` (- (`self.Health`) Damage))
  (if (<= (`self.Health`) 0.0)
    ;[1 1 1] Mort
    (`PrimitiveComponent.SetSimulatePhysics` (`self.Mesh`) true)
    (`CharacterMovementComponent.DisableMovement` (`self.CharacterMovement`))
    (`PrimitiveComponent.SetCollisionEnabled` (`self.CapsuleComponent`) "QueryOnly")
    (`KismetSystemLibrary.Delay` 5.0)
    (`self.K2_DestroyActor`)
    (else
      (`PrimitiveComponent.SetMaterial` (`self.Mesh`) 0 "/Game/Game/2D/M_Damage.M_Damage")
      (`KismetSystemLibrary.Delay` 0.1)
      (`PrimitiveComponent.SetMaterial` (`self.Mesh`) 0 "/Game/Game/Meshes/TestHippo/Material_001.Material_001"))))

(event `self.OnLanded`
  (params (Hit :type "HitResult Structure (by ref)"))
  (`GameplayStatics.PlayWorldCameraShake` "/Game/Game/BP_Kadmerad.BP_Kadmerad_C" (`self.K2_GetActorLocation` (`GameplayStatics.GetPlayerCharacter` 0)) 1000.0 100000.0)
  (`KismetSystemLibrary.Delay` 1.0)
  (`PrimitiveComponent.SetCollisionEnabled` (`self.Detection`) "QueryOnly"))

(event `self.Detection.OnComponentBeginOverlap`
  (params (OverlappedComponent :type "PrimitiveComponent Object Reference") (OtherActor :type "Actor Object Reference") (OtherComp :type "PrimitiveComponent Object Reference") (OtherBodyIndex :type Integer) (bFromSweep :type Boolean) (SweepResult :type "HitResult Structure (by ref)"))
  (if (`self.ShouldStomp`)
    (set `self.ShouldJump` false)
    (cast `/Game/Game/BP_ThirdPersonCharacter` OtherActor)
    (`SkeletalMeshComponent.PlayAnimation` (`self.Mesh`) "/Game/Game/Meshes/TestHippo/HippoStomp.HippoStomp" false)
    (`KismetSystemLibrary.Delay` 0.8)
    (if (`self.ShouldStomp`)
      (`PrimitiveComponent.SetCollisionEnabled` (`self.HitZone`) "QueryOnly")
      (set `self.ShouldJump` true))))

(event `self.Detection.OnComponentEndOverlap`
  (params (OverlappedComponent :type "PrimitiveComponent Object Reference") (OtherActor :type "Actor Object Reference") (OtherComp :type "PrimitiveComponent Object Reference") (OtherBodyIndex :type Integer))
  (cast `/Game/Game/BP_ThirdPersonCharacter` OtherActor))

(event `self.HitZone.OnComponentBeginOverlap`
  (params (OverlappedComponent :type "PrimitiveComponent Object Reference") (OtherActor :type "Actor Object Reference") (OtherComp :type "PrimitiveComponent Object Reference") (OtherBodyIndex :type Integer) (bFromSweep :type Boolean) (SweepResult :type "HitResult Structure (by ref)")))

(fn `UserConstructionScript`)