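; BP_Lilypad1 is a lilypad actor that moves its Cylinder component along a spline when the GoSpline event is called.
; GoSpline sets the timeline play rate to the inverse of Durée and plays it from the start.
; Each update converts the Pourcentage track into a distance along the spline and moves the cylinder to that world position, without sweep.
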(event `GoSpline`
  (bind _spline (`self.Spline`))
  (`TimelineComponent.SetPlayRate` (`self.Timeline`) (/ 1.0 (`self.Durée`)))
  (bind (_direction _pourcentage) (`Timeline|Timeline` :!via `PlayFromStart`)
    (:`Update`
      (`SceneComponent.K2_SetWorldLocation` (`self.Cylinder`) (`SplineComponent.GetLocationAtDistanceAlongSpline` _spline (* _pourcentage (`SplineComponent.GetSplineLength` _spline)) "World") false false))))

(fn `UserConstructionScript`)