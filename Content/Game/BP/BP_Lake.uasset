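; BP_Lake is a lake hazard that sends the player to the game-over level when the third-person character overlaps its Cylinder.
; Its LakeUp event calls GoSpline on every BP_Lilypad1_Child and, within the same loop, eases the Cylinder to a raised relative height.
; BeginPlay caches a BP_Lilypad2_Child reference, which this graph does not use further.
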(event `self.ReceiveBeginPlay`
  (bind _returnvalue (`GameplayStatics.GetActorOfClass` "/Game/Game/BP/BP_Lilypad2_Child.BP_Lilypad2_Child_C"))
  (set `self.Lilypad2C` _returnvalue))

(event `self.ReceiveTick`
  (params (DeltaSeconds :type "Float (single-precision)")))

(event `self.Cylinder.OnComponentBeginOverlap`
  (params (OverlappedComponent :type "PrimitiveComponent Object Reference") (OtherActor :type "Actor Object Reference") (OtherComp :type "PrimitiveComponent Object Reference") (OtherBodyIndex :type Integer) (bFromSweep :type Boolean) (SweepResult :type "HitResult Structure (by ref)"))
  ;[1 1 1] Dead player
  (cast `/Game/Game/BP_ThirdPersonCharacter` OtherActor)
  (`GameplayStatics.OpenLevelBySoftObjectPtr` "/Game/Game/Levels/L_GameOver.L_GameOver"))

(event `LakeUp`
  (bind _outactors (`GameplayStatics.GetAllActorsOfClass` "/Game/Game/BP/BP_Lilypad1_Child.BP_Lilypad1_Child_C"))
  (for _array_element _outactors
    (`/Game/Game/BP/BP_Lilypad.GoSpline` _array_element)
    (`KismetSystemLibrary.MoveComponentTo` (`self.Cylinder`) (0.0 0.0 250.0) (struct) true true 1.0)))

(fn `UserConstructionScript`)