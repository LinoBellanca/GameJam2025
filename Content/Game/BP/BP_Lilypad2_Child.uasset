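; BP_Lilypad2_Child is a child lilypad Blueprint that rises on demand and sets BP_Lilypad1_Child actors moving.
; Its NenuUp event calls GoSpline on every BP_Lilypad1_Child in the level and, inside that same loop, eases its own Cylinder to a fixed raised relative position.
; The construction script runs the parent's, then applies the InClosedLoop setting to the Spline.
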(event `self.ReceiveTick`
  (params (DeltaSeconds :type "Float (single-precision)"))
  (`parent.ReceiveTick` DeltaSeconds))

(event `NenuUp`
  (bind _outactors (`GameplayStatics.GetAllActorsOfClass` "/Game/Game/BP/BP_Lilypad1_Child.BP_Lilypad1_Child_C"))
  (for _array_element _outactors
    (`self.GoSpline` _array_element)
    (`KismetSystemLibrary.MoveComponentTo` (`self.Cylinder`) (0.0 0.0 125.0) (struct) true true 1.0)))

(fn `UserConstructionScript`
  (`parent.UserConstructionScript`)
  (`SplineComponent.SetClosedLoop` (`self.Spline`) (`self.In Closed Loop`) true))