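; Special enemy Blueprint that chases the player and, using a heron attack montage, fires fish projectiles from its mouth.
; Tick reissues AIMoveTo toward the player character every frame.
; Detection overlap zeroes walk speed and starts a delayed montage-and-spawn attack loop, while leaving stops the montage and restores movement.
; Damage reduces health after a brief delay; at zero it ragdolls, disables capsule collision and movement, then is destroyed.
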(event `self.ReceiveBeginPlay`)

(event `self.ReceiveTick`
  (params (DeltaSeconds :type "Float (single-precision)"))
  (bind _returnvalue (`GameplayStatics.GetPlayerCharacter` 0))
  (bind (_returnvalue_x _returnvalue_y) (`KismetMathLibrary.BreakVector` (`self.K2_GetActorLocation` _returnvalue)))
  (`|ExecutionSequence`
    (:`then_0`
      (`|AIMoveTo` self (`KismetMathLibrary.MakeVector` _returnvalue_x _returnvalue_y) _returnvalue 100.0))))

(event `self.ReceiveAnyDamage`
  (params (Damage :type "Float (single-precision)") (DamageType :type "DamageType Object Reference") (InstigatedBy :type "Controller Object Reference") (DamageCauser :type "Actor Object Reference"))
  ;[1 1 1] Dégât reçu
  (`KismetSystemLibrary.Delay` 0.1)
  (set `self.Health` (- (`self.Health`) Damage))
  (if (<= (`self.Health`) 0.0)
    ;[1 1 1] Mort
    (`PrimitiveComponent.SetSimulatePhysics` (`self.Mesh`) true)
    (`CharacterMovementComponent.DisableMovement` (`self.CharacterMovement`))
    (`PrimitiveComponent.SetCollisionEnabled` (`self.CapsuleComponent`) "NoCollision")
    (`KismetSystemLibrary.Delay` 5.0)
    (`self.K2_DestroyActor`)))

(event `self.Detection.OnComponentBeginOverlap`
  (params (OverlappedComponent :type "PrimitiveComponent Object Reference") (OtherActor :type "Actor Object Reference") (OtherComp :type "PrimitiveComponent Object Reference") (OtherBodyIndex :type Integer) (bFromSweep :type Boolean) (SweepResult :type "HitResult Structure (by ref)"))
  (bind _asbp_third_person_character (cast `/Game/Game/BP_ThirdPersonCharacter` OtherActor))
  (set `self.Target` _asbp_third_person_character)
  (set `self.ShouldAttack` true)
  (set `CharacterMovementComponent.MaxWalkSpeed` 0.0 (`self.CharacterMovement`))
  (`KismetSystemLibrary.Delay` 3.0 :!label _label)
  (if (`self.ShouldAttack`)
    (`self.PlayAnimMontage` "/Game/Game/Meshes/TestHeron/HeronAttack_Montage.HeronAttack_Montage")
    (`KismetSystemLibrary.Delay` 1.2)
    (`|SpawnActorFromClass` "/Game/Game/BP_FishBullet.BP_FishBullet_C" (`SceneComponent.K2_GetComponentToWorld` (`self.Mouth`)) "Undefined" "MultiplyWithRoot" null null)
    (if (`self.ShouldAttack`)
      (goto _label)
      (else
        (set `CharacterMovementComponent.MaxWalkSpeed` 300.0 (`self.CharacterMovement`))))))

(event `self.Detection.OnComponentEndOverlap`
  (params (OverlappedComponent :type "PrimitiveComponent Object Reference") (OtherActor :type "Actor Object Reference") (OtherComp :type "PrimitiveComponent Object Reference") (OtherBodyIndex :type Integer))
  (cast `/Game/Game/BP_ThirdPersonCharacter` OtherActor)
  (set `self.ShouldAttack` false)
  (`self.StopAnimMontage` "/Game/Game/Meshes/TestHeron/HeronAttack_Montage.HeronAttack_Montage")
  (set `CharacterMovementComponent.MaxWalkSpeed` 400.0 (`self.CharacterMovement`)))

(fn `UserConstructionScript`)