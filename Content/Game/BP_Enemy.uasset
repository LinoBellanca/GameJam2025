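; Enemy character Blueprint that chases the player and dies when its health runs out.
; Tick re-issues AIMoveTo toward player 0 every frame and prints current Health as debug output.
; AnyDamage subtracts damage after a brief Delay, so hits landing during that wait are not applied.
; At zero health it turns the mesh to physics, disables movement and capsule collision, then destroys itself after a pause.
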(event `self.ReceiveBeginPlay`)

(event `self.ReceiveTick`
  (params (DeltaSeconds :type "Float (single-precision)"))
  (bind _returnvalue (`GameplayStatics.GetPlayerCharacter` 0))
  (bind (_returnvalue_x _returnvalue_y) (`KismetMathLibrary.BreakVector` (`self.K2_GetActorLocation` _returnvalue)))
  (`|ExecutionSequence`
    (:`then_0`
      (`|AIMoveTo` self (`KismetMathLibrary.MakeVector` _returnvalue_x _returnvalue_y) _returnvalue 100.0))
    (:`then_1`
      (`KismetSystemLibrary.PrintString` (`KismetStringLibrary.Conv_DoubleToString` (`self.Health`))))))

(event `self.ReceiveAnyDamage`
  (params (Damage :type "Float (single-precision)") (DamageType :type "DamageType Object Reference") (InstigatedBy :type "Controller Object Reference") (DamageCauser :type "Actor Object Reference"))
  ;[1 1 1] Dégât reçu
  (`KismetSystemLibrary.Delay` 0.1)
  (set `self.Health` (- (`self.Health`) Damage))
  (if (<= (`self.Health`) 0.0)
    ;[1 1 1] Mort
    (`PrimitiveComponent.SetSimulatePhysics` (`self.Mesh`) true)
    (`CharacterMovementComponent.DisableMovement` (`self.CharacterMovement`))
    (`PrimitiveComponent.SetCollisionEnabled` (`self.CapsuleComponent`) "NoCollision")
    (`KismetSystemLibrary.Delay` 5.0)
    (`self.K2_DestroyActor`)))

(fn `UserConstructionScript`)